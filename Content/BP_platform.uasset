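; BP_platform is a moving platform that slides its Cube between its local origin and a configurable EndLocation.
; On BeginPlay it sets the Movement timeline's play rate from Speed, then starts it after a short delay.
; The timeline, intended to loop, feeds its Smart track into a vector lerp that sets the Cube's relative location without sweeping.
; The Box overlap event has no effect, and its player-character check is unused.
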(event OnComponentBeginOverlap(Box)
  (params (OverlappedComponent :type Primitive%20Component%20Object%20Reference) (OtherActor :type Actor%20Object%20Reference) (OtherComp :type Primitive%20Component%20Object%20Reference) (OtherBodyIndex :type Integer) (bFromSweep :type Boolean) (SweepResult :type Hit%20Result%20Structure%20%28by%20ref%29))
  (if true
    _))

(event EventBeginPlay
  ;[1 1 1] set movement function and the movement speed
  (Components|Timeline|SetPlayRate (Variables|Default|Getmovement) (Variables|Default|Getspeed))
  (Utilities|FlowControl|Delay 0.5)
  ;[1 1 1] make the timeline of movement and make a loop
  (bind _smart (Timeline|movement Play)
    (:Update
      ;[1 1 1] set end location
      (Transformation|SetRelativeLocation (Variables|Default|GetCube) (Math|Vector|Lerp(Vector) "0, 0, 0" (Variables|Default|Getend%20location) _smart) false false))))

(fn ConstructionScript)