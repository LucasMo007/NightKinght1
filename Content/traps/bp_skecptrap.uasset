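; Spike trap that animates when triggered and kills the player on contact with its death volume.
; Entering the trigger collision plays the skeletal spike animation once; leaving sets a negative play rate to run it backward.
; The death trigger destroys player character 0 without checking what overlapped, then after a short delay opens a hard-coded level by name.
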(event OnComponentBeginOverlap(triggercollision)
  (params (OverlappedComponent :type Primitive%20Component%20Object%20Reference) (OtherActor :type Actor%20Object%20Reference) (OtherComp :type Primitive%20Component%20Object%20Reference) (OtherBodyIndex :type Integer) (bFromSweep :type Boolean) (SweepResult :type Hit%20Result%20Structure%20%28by%20ref%29))
  (Components|Animation|PlayAnimation (Variables|Default|Getspaketrap) "/Game/traps/Sk_spiketrap_Anim.Sk_spiketrap_Anim" false))

(event OnComponentEndOverlap(triggercollision)
  (params (OverlappedComponent :type Primitive%20Component%20Object%20Reference) (OtherActor :type Actor%20Object%20Reference) (OtherComp :type Primitive%20Component%20Object%20Reference) (OtherBodyIndex :type Integer))
  (Components|Timeline|SetPlayRate (Variables|Default|Getspaketrap) -1.0)
  (Audio|Components|Audio|Play (Variables|Default|Getspaketrap) false))

(event OnComponentBeginOverlap(deathdrigger)
  (params (OverlappedComponent :type Primitive%20Component%20Object%20Reference) (OtherActor :type Actor%20Object%20Reference) (OtherComp :type Primitive%20Component%20Object%20Reference) (OtherBodyIndex :type Integer) (bFromSweep :type Boolean) (SweepResult :type Hit%20Result%20Structure%20%28by%20ref%29))
  (Actor|DestroyActor (Game|GetPlayerCharacter 0))
  (Utilities|FlowControl|Delay 0.2)
  (Game|OpenLevel(byName) "animation_lucas_3-6"))

(event EventBeginPlay)

(event Collision|EventActorBeginOverlap
  (params (OtherActor :type Actor%20Object%20Reference)))

(event EventTick
  (params (DeltaSeconds :type Float%20%28single-precision%29)))

(fn ConstructionScript)