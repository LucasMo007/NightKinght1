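; Skeleton enemy character that fights the player with a socket-attached sword and supports lock-on targeting.
; Runs a behavior tree steered by a blackboard behaviour enum, which pawn sensing, damage and sphere exit update.
; Hits show the health bar and play a stagger montage; death stops AI, disables collision and releases player lock-on.
; Attacks play random montages, with a trace component holding the sword reference and enemy-tagged actors.
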(event OnSeePawn(PawnSensing)
  (params (Pawn :type Pawn%20Object%20Reference))
  ;[1 1 1] Handle enemy vision
  (if (and (== Pawn (Game|GetPlayerCharacter 0)) (Utilities|Enum|NotEqual(Enum) (Variables|Default|Getbehaviour) "NewEnumerator0"))
    (Variables|Default|Setbehaviour "NewEnumerator3")
    (AI|Components|Blackboard|SetValueasEnum (AI|GetBlackboard 0) (Utilities|Name|MakeLiteralName "ebehaviour") (Variables|Default|Getbehaviour))))

(event OnComponentEndOverlap(Sphere)
  (params (OverlappedComponent :type Primitive%20Component%20Object%20Reference) (OtherActor :type Actor%20Object%20Reference) (OtherComp :type Primitive%20Component%20Object%20Reference) (OtherBodyIndex :type Integer))
  ;[1 1 1] Escape enemy
  (Utilities|Casting|CastToBP_ThirdPersonCharacter OtherActor)
  (Variables|Default|Setbehaviour "NewEnumerator1")
  (AI|Components|Blackboard|SetValueasEnum (AI|GetBlackboard 0) (Utilities|Name|MakeLiteralName "ebehaviour") (Variables|Default|Getbehaviour))
  (Rendering|SetVisibility (Variables|Default|Gethealthbar) false false))

(event Custom|Attack
  ;[1 1 1] Attack system
  (bind _returnvalue (Animation|PlayAnimMontage (.OutItem (Utilities|Array|Random (Variables|Default|Getattackanimations))) 1.0 "None"))
  (Variables|Default|Setattacklength _returnvalue))

(event Custom|Clear%20hit%20actors
  ;[1 1 1] clear hit actors
  (Utilities|Array|Clear (Variables|/Game/Equipment/TraceComponent.TraceComponent_C|Getactorstoignore (Variables|Default|GetTraceComponent))))

(event EventBeginPlay
  ;[1 1 1] Set up enemy character
  (Variables|Default|Setmaxhealth (Variables|Default|Gethealth))
  (AI|RunBehaviorTree (AI|GetAIController self) "/Game/Enemy/BehaviourTree/Skeleton_BT.Skeleton_BT")
  (bind _returnvalue (Game|SpawnActorfromClass (Variables|Default|Getsword) (Transformation|GetSocketTransform (Variables|Character|GetMesh) "sword" "RTS_World") "Undefined" "SelectDefaultAtRuntime" 0 0))
  (bind _output_get (Variables|Default|Setswordref _returnvalue))
  (Transformation|AttachComponentToComponent _output_get (Variables|Character|GetMesh) "sword" "SnapToTarget" "SnapToTarget" "SnapToTarget" true)
  (Variables|/Game/Equipment/TraceComponent.TraceComponent_C|Setswordref (Variables|Default|GetTraceComponent) (Variables|Default|Getswordref))
  (bind _asbp_third_person_character (Utilities|Casting|CastToBP_ThirdPersonCharacter (Game|GetPlayerCharacter 0)))
  (Variables|Default|Setplayerref _asbp_third_person_character)
  (AI|Components|Blackboard|SetValueasEnum (AI|GetBlackboard 0) (Utilities|Name|MakeLiteralName "ebehaviour") (Variables|Default|Getbehaviour))
  (Variables|/Game/Equipment/RotatingComponent.RotatingComponent_C|SetTarget (Variables|Default|GetRotatingComponent) (Game|GetPlayerCharacter 0))
  (bind _outactors (Actor|GetAllActorswithTag "enemy"))
  (Variables|/Game/Equipment/TraceComponent.TraceComponent_C|Setenemy (Variables|Default|GetTraceComponent) _outactors)
  (bind _asskeleton_health_bar_wb (Utilities|Casting|CastToSkeletonHealthBar_WB (UserInterface|GetWidget (Variables|Default|Gethealthbar))))
  (bind _output_get_2 (Variables|Default|Sethealthbarref _asskeleton_health_bar_wb))
  (Variables|/Game/Enemy/Blueprints/SkeletonHealthBar_WB.SkeletonHealthBar_WB_C|Setskeletonref _output_get_2 self))

(event Game|Damage|EventAnyDamage
  (params (Damage :type Float%20%28single-precision%29) (DamageType :type Damage%20Type%20Object%20Reference) (InstigatedBy :type Controller%20Object%20Reference) (DamageCauser :type Actor%20Object%20Reference))
  (bind _playerref (Variables|Default|Getplayerref))
  (bind _targetactor (Variables|/Game/ThirdPerson/Blueprints/BP_ThirdPersonCharacter.BP_ThirdPersonCharacter_C|GetTargetactor _playerref))
  ;[1 1 1] Damage system
  (Variables|Default|Setbehaviour "NewEnumerator0")
  (AI|Components|Blackboard|SetValueasEnum (AI|GetBlackboard 0) (Utilities|Name|MakeLiteralName "ebehaviour") (Variables|Default|Getbehaviour))
  (bind _output_get (Variables|Default|Sethealth (- (Variables|Default|Gethealth) Damage)))
  (if (<= _output_get 0.0)
    (Utilities|FlowControl|DoOnce false
      (:Completed
        (Collision|SetCollisionEnabled (Variables|Collision|GetCapsuleComponent) "NoCollision")
        (Rendering|SetVisibility (Variables|Default|Gethealthbar) false false)
        (AI|Logic|StopLogic (Variables|/Script/AIModule.AIController|GetBrainComponent (AI|GetAIController self)) "die")
        (Variables|Default|Setenemydead? true)
        (Animation|PlayAnimMontage "/Game/Enemy/Animations/SkeleDeath_Montage.SkeleDeath_Montage" 1.0 "None")
        (Utilities|IsValid _targetactor
          (:Is%20Valid
            (if (== _targetactor self)
              (Default|Disengagelockon (Variables|Default|Getplayerref)))))))
    (else
      (Rendering|SetVisibility (Variables|Default|Gethealthbar) true false)
      (Default|Updatehealthbar (Variables|Default|Gethealthbarref))
      (Components|Movement|StopMovementImmediately (Variables|Character|GetCharacterMovement))
      (bind _returnvalue (Animation|PlayAnimMontage "/Game/Enemy/Animations/Skele_Hit_Montage.Skele_Hit_Montage" 1.0 "None"))
      (Utilities|FlowControl|RetriggerableDelay _returnvalue)
      (Variables|Default|Setbehaviour "NewEnumerator3")
      (AI|Components|Blackboard|SetValueasEnum (AI|GetBlackboard 0) (Utilities|Name|MakeLiteralName "ebehaviour") (Variables|Default|Getbehaviour)))))

(event EventOnselected
  ;[1 1 1] Handle lock on
  (Rendering|SetVisibility (Variables|Default|GetLockon) true false))

(event EventOndeselected
  ;[1 1 1] Handle lock on
  (Rendering|SetVisibility (Variables|Default|GetLockon) false false))

(fn ConstructionScript)

(fn Isdead
  (return (Variables|Default|Getenemydead?)))